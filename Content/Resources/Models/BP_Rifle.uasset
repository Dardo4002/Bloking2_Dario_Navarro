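; BP_Rifle is a rifle weapon Blueprint that fires a hitscan shot from the first-person character's camera.
; Disparar runs a debug-drawn line trace against WorldStatic objects and spawns a temporary AmmoLight at the impact point.
; A CanShoot flag gates firing, re-arming after a half-second delay only on a blocking hit, when the light is also destroyed.
; The construction script applies MyColor to the mesh's BodyColor material parameter.
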(event `Disparar`
  (if (`self.CanShoot`)
    (set `self.CanShoot` false)
    (`KismetSystemLibrary.PrintString` "Rifle")
    (bind _asbp_first_person_character (cast `/Game/FirstPerson/Blueprints/BP_FirstPersonCharacter` (`GameplayStatics.GetPlayerCharacter` 0)))
    (bind _firstpersoncamera (`/Game/FirstPerson/Blueprints/BP_FirstPersonCharacter.FirstPersonCamera` _asbp_first_person_character))
    (bind _returnvalue (`SceneComponent.K2_GetComponentLocation` _firstpersoncamera))
    (bind (_outhit _returnvalue_2) (`KismetSystemLibrary.LineTraceSingleForObjects` :`Start` _returnvalue :`End` (+ _returnvalue (* (`SceneComponent.GetForwardVector` _firstpersoncamera) (`self.Raylegnth`))) :`ObjectTypes` (`|MakeArray` "ObjectTypeQuery1" :!type "EObjectTypeQuery Enum") :`DrawDebugType` "ForDuration"))
    (if _returnvalue_2
      (bind (_bblockinghit _binitialoverlap _time _distance _location _impactpoint) (`GameplayStatics.BreakHitResult` _outhit))
      (if _bblockinghit
        (bind _returnvalue_3 (`|SpawnActorFromClass` "/Game/FPWeapon/AmmoLight.AmmoLight_C" (`KismetMathLibrary.MakeTransform` _impactpoint) "AdjustIfPossibleButAlwaysSpawn" "MultiplyWithRoot" null null))
        (`KismetSystemLibrary.Delay` 0.5)
        (set `self.CanShoot` true)
        (`/Game/FPWeapon/AmmoLight.Destroy` _returnvalue_3)))))

(fn `UserConstructionScript`
  (`MeshComponent.SetVectorParameterValueOnMaterials` (`self.SkeletalMesh`) "BodyColor" (`KismetMathLibrary.Conv_LinearColorToVector` (`self.MyColor`))))