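; Interactive sliding door that opens and closes when an interactor triggers its Interact F function.
; Interact F picks OpenDoor or CloseDoor from the Closed flag, playing or reversing a single timeline, and returns true.
; The timeline track, scaled by FDistance, drives the door mesh's relative Y position.
; Closed flips only when the timeline finishes, so interacting mid-motion does not change direction.
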(event `OpenDoor`
  (bind (_direction _operdoor) (`Timeline|Timeline` :!label _label)
    (:`Update`
      (`SceneComponent.K2_SetRelativeLocation` (`self.SM_Door`) (`KismetMathLibrary.MakeVector` 0.0 (* _operdoor (`self.F_Distance`))) false false))
    (:`Finished`
      (set `self.Closed` (not (`self.Closed`))))))

(event `CloseDoor`
  (goto _label :!via `Reverse`))

(fn `Interact F`
  (params (Interactor :type "Character Object Reference"))
  (returns (`Interaction?` :type Boolean))
  (if (`self.Closed`)
    (`self.OpenDoor`)
    (else
      (`self.CloseDoor`)))
  (return true))

(fn `UserConstructionScript`)