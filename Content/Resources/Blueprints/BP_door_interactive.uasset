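; Interactive door Blueprint that swings its door mesh open or closed when an interactor calls InteractF.
; The TL_open timeline drives the mesh's relative yaw scaled by FAngle, playing to open and reversing to close.
; InteractF picks the direction from the Closed flag, which flips only when the timeline finishes, and always returns true.
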(event `OpenDoor`
  (bind (_direction _operdoor) (`Timeline|TL_open` :!label _label)
    (:`Update`
      (`SceneComponent.K2_SetRelativeRotation` (`self.SM_door`) (`KismetMathLibrary.MakeRotator` 0.0 0.0 (* _operdoor (`self.F_angle`))) false false))
    (:`Finished`
      (set `self.Closed` (not (`self.Closed`))))))

(event `CloseDoor`
  (goto _label :!via `Reverse`))

(fn `Interact F`
  (params (Interactor :type "Character Object Reference"))
  (returns (`Interaction?` :type Boolean))
  (if (`self.Closed`)
    (`self.OpenDoor`)
    (else
      (`self.CloseDoor`)))
  (return true))

(fn `UserConstructionScript`)