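; Key1 is a collectible key pickup that adds to the first-person character's key count.
; Its Trigger overlap shows a WB_MessageInteract prompt while the character is in range and removes it on exit.
; The InteractF function increments KeyCount while it is below four, spawns the PS_GrabItem Niagara effect at the key's location and destroys the actor.
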(event `self.ReceiveBeginPlay`)

(event `self.Trigger.OnComponentBeginOverlap`
  (params (OverlappedComponent :type "PrimitiveComponent Object Reference") (OtherActor :type "Actor Object Reference") (OtherComp :type "PrimitiveComponent Object Reference") (OtherBodyIndex :type Integer) (bFromSweep :type Boolean) (SweepResult :type "HitResult Structure (by ref)"))
  (cast `/Game/FirstPerson/Blueprints/BP_FirstPersonCharacter` OtherActor)
  (bind _returnvalue (`|CreateWidget` "/Game/Resources/Widgets/WB_MessageInteract.WB_MessageInteract_C"))
  (`UserWidget.AddToViewport` _returnvalue 0))

(event `self.Trigger.OnComponentEndOverlap`
  (params (OverlappedComponent :type "PrimitiveComponent Object Reference") (OtherActor :type "Actor Object Reference") (OtherComp :type "PrimitiveComponent Object Reference") (OtherBodyIndex :type Integer))
  (cast `/Game/FirstPerson/Blueprints/BP_FirstPersonCharacter` OtherActor)
  (`Widget.RemoveFromParent` (stale `self.Trigger.OnComponentBeginOverlap` _returnvalue)))

(fn `Interact F`
  (params (Interactor :type "Character Object Reference"))
  (returns (`Interaction?` :type Boolean))
  (bind _asbp_first_person_character (cast `/Game/FirstPerson/Blueprints/BP_FirstPersonCharacter` Interactor))
  (if (not (>= (`/Game/FirstPerson/Blueprints/BP_FirstPersonCharacter.key_count` _asbp_first_person_character) 4))
    (bind _result (`/Engine/EditorBlueprintResources/StandardMacros.IncrementInt` (`/Game/FirstPerson/Blueprints/BP_FirstPersonCharacter.key_count` _asbp_first_person_character))
      (:`  `
        (set `/Game/FirstPerson/Blueprints/BP_FirstPersonCharacter.key_count` _result _asbp_first_person_character)
        (`AddComponent|NODE_AddNiagaraComponent-0`)
        (`NiagaraFunctionLibrary.SpawnSystemAtLocation` "/Game/Particles/PS_GrabItem.PS_GrabItem" (`SceneComponent.K2_GetComponentLocation` (`self.key`)))
        (`self.K2_DestroyActor`)
        (return false)))))

(fn `UserConstructionScript`)