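; Interactive locked door that the first-person character opens by spending a key.
; A trigger overlap checks the player's key count against CantidadLlaves and shows an interact or no-key widget, removed on exit.
; InteractF calls OpenDoor, which deducts one key and rotates the mesh's yaw through a timeline, or CloseDoor, which reverses it.
; The timeline's finish assigns Closed to itself, so the open/closed state never toggles here.
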(event `OpenDoor`
  ;[1 1 1] Comprueba la llave y reduce el número
  (bind _asbp_first_person_character (cast `/Game/FirstPerson/Blueprints/BP_FirstPersonCharacter` (stale `self.Trigger.OnComponentBeginOverlap` OtherActor)))
  (if (>= (`/Game/FirstPerson/Blueprints/BP_FirstPersonCharacter.key_count` _asbp_first_person_character) (`self.CantidadLlaves`))
    (bind _result (`/Engine/EditorBlueprintResources/StandardMacros.DecrementInt` (`/Game/FirstPerson/Blueprints/BP_FirstPersonCharacter.key_count` _asbp_first_person_character))
      (:`  `
        (set `/Game/FirstPerson/Blueprints/BP_FirstPersonCharacter.key_count` _result _asbp_first_person_character)
        (if (`self.Closed`)
          ;[1 1 1] Abre y cierra la puerta
          (bind (_direction _operdoor) (`Timeline|TL_open` :!label _label)
            (:`Update`
              (`SceneComponent.K2_SetRelativeRotation` (`self.SM_door`) (`KismetMathLibrary.MakeRotator` 0.0 0.0 (* _operdoor (`self.F_angle`))) false false))
            (:`Finished`
              (set `self.Closed` (`self.Closed`)))))))))

(event `CloseDoor`
  (goto _label :!via `Reverse`))

(event `self.Trigger.OnComponentBeginOverlap`
  (params (OverlappedComponent :type "PrimitiveComponent Object Reference") (OtherActor :type "Actor Object Reference") (OtherComp :type "PrimitiveComponent Object Reference") (OtherBodyIndex :type Integer) (bFromSweep :type Boolean) (SweepResult :type "HitResult Structure (by ref)"))
  ;[1 1 1] Detectar jugador
  (bind _asbp_first_person_character (cast `/Game/FirstPerson/Blueprints/BP_FirstPersonCharacter` OtherActor))
  ;[1 1 1] Comprobar llave
  (if (>= (`/Game/FirstPerson/Blueprints/BP_FirstPersonCharacter.key_count` _asbp_first_person_character) (`self.CantidadLlaves`))
    (if (`self.Closed`)
      ;[1 1 1] Crear y quitar widget
      (bind _returnvalue (`|CreateWidget` "/Game/Resources/Widgets/WB_MessageInteract.WB_MessageInteract_C"))
      (`UserWidget.AddToViewport` _returnvalue 0))
    (elif (`self.Closed`)
      (bind _returnvalue_2 (`|CreateWidget` "/Game/Resources/Widgets/WB_NoKey.WB_NoKey_C"))
      (`UserWidget.AddToViewport` _returnvalue_2 0))))

(event `self.Trigger.OnComponentEndOverlap`
  (params (OverlappedComponent :type "PrimitiveComponent Object Reference") (OtherActor :type "Actor Object Reference") (OtherComp :type "PrimitiveComponent Object Reference") (OtherBodyIndex :type Integer))
  ;[1 1 1] Detectar jugador
  (bind _asbp_first_person_character (cast `/Game/FirstPerson/Blueprints/BP_FirstPersonCharacter` OtherActor))
  ;[1 1 1] Comprobar llave
  (if (>= (`/Game/FirstPerson/Blueprints/BP_FirstPersonCharacter.key_count` _asbp_first_person_character) (`self.CantidadLlaves`))
    (if (`self.Closed`)
      ;[1 1 1] Crear y quitar widget
      (`Widget.RemoveFromParent` (stale `self.Trigger.OnComponentBeginOverlap` _returnvalue) :!label _label_2))
    (else
      (`Widget.RemoveFromParent` (stale `self.Trigger.OnComponentBeginOverlap` _returnvalue_2))
      (goto _label_2))))

(fn `Interact F`
  (params (Interactor :type "Character Object Reference"))
  (returns (`Interaction?` :type Boolean))
  (if (`self.Closed`)
    (`self.OpenDoor`)
    (else
      (`self.CloseDoor`)))
  (return true))

(fn `UserConstructionScript`)