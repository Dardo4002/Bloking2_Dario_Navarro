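; A double door Blueprint that swings open when the first-person character enters its trigger and closes when they leave.
; Trigger overlap events cast to BP_FirstPersonCharacter, then play or reverse the Timer timeline.
; The timeline's OpenDoor track scales a separate angle variable for each door mesh to set its relative yaw, with SMDoor1 offset by a half turn to mirror the other leaf.
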(event `self.Trigger.OnComponentBeginOverlap`
  (params (OverlappedComponent :type "PrimitiveComponent Object Reference") (OtherActor :type "Actor Object Reference") (OtherComp :type "PrimitiveComponent Object Reference") (OtherBodyIndex :type Integer) (bFromSweep :type Boolean) (SweepResult :type "HitResult Structure (by ref)"))
  (cast `/Game/FirstPerson/Blueprints/BP_FirstPersonCharacter` OtherActor)
  (bind (_direction _open_door) (`Timeline|Timer` :!label _label)
    (:`Update`
      (`SceneComponent.K2_SetRelativeRotation` (`self.SM_Door1`) (`KismetMathLibrary.MakeRotator` 0.0 0.0 (+ (* _open_door (`self.F_Angle`)) 180.0)) false false)
      (`SceneComponent.K2_SetRelativeRotation` (`self.SM_Door`) (`KismetMathLibrary.MakeRotator` 0.0 0.0 (* _open_door (`self.F_Angle_0`))) false false))))

(event `self.Trigger.OnComponentEndOverlap`
  (params (OverlappedComponent :type "PrimitiveComponent Object Reference") (OtherActor :type "Actor Object Reference") (OtherComp :type "PrimitiveComponent Object Reference") (OtherBodyIndex :type Integer))
  (cast `/Game/FirstPerson/Blueprints/BP_FirstPersonCharacter` OtherActor)
  (goto _label :!via `Reverse`))

(fn `UserConstructionScript`)