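; BP_Rifle2 is a rifle Blueprint that fires AmmoStunt projectiles through its Disparar event.
; Disparar prints a debug string, spawns ammo at Aimpoint and sets its Sphere's physics velocity along the actor-to-spawn direction, scaled by ThrowForce.
; The spawned ammo is destroyed immediately afterward, with no delay.
; The construction script tints the skeletal mesh's BodyColor material parameter from MyColor.
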(event `Disparar`
  (`KismetSystemLibrary.PrintString` "Disparo")
  (bind _returnvalue (`|SpawnActorFromClass` "/Game/FPWeapon/AmmoStunt.AmmoStunt_C" (`KismetMathLibrary.MakeTransform` (`SceneComponent.K2_GetComponentLocation` (`self.Aimpoint`)) (`self.K2_GetActorRotation`)) "Undefined" "MultiplyWithRoot" null null))
  (`PrimitiveComponent.SetPhysicsLinearVelocity` (`/Game/FPWeapon/AmmoStunt.Sphere` _returnvalue) (* (`KismetMathLibrary.GetDirectionUnitVector` (`self.K2_GetActorLocation`) (`self.K2_GetActorLocation` _returnvalue)) (`self.throwForce`)) false "None")
  (`/Game/FPWeapon/AmmoStunt.Destroy` _returnvalue))

(fn `UserConstructionScript`
  (`MeshComponent.SetVectorParameterValueOnMaterials` (`self.SkeletalMesh`) "BodyColor" (`KismetMathLibrary.Conv_LinearColorToVector` (`self.MyColor`))))